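; GS_Domination is the game state for a Domination mode, handling the mode's score overlay.
; When the overlay is requested, it creates a WB_Dominion widget, adds it to the viewport and sets the bar maximum to the points needed to win.
; Team point updates trigger an overlay update, which passes the game state to the widget to refresh its bar.
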(event `self.ReceiveBeginPlay`
  (`parent.ReceiveBeginPlay`))

(event `self.PopGameModeOverlay`
  (bind _returnvalue (`|CreateWidget` "/Game/Blueprints/UI/WB_Dominion.WB_Dominion_C"))
  (bind _output_get (set `self.DominationWidget` _returnvalue))
  (`UserWidget.AddToViewport` _output_get 0)
  (set `/Game/Blueprints/UI/WB_Dominion.maxBarValue` (`self.PointToWin`) _output_get))

(event `self.OnTeamPointUpdate`
  (`self.OnTeamOverlayUpdate`))

(event `self.OnTeamOverlayUpdate`
  (`/Game/Blueprints/UI/WB_Dominion.UpdateBar` (`self.DominationWidget`) self))

(fn `UserConstructionScript`)