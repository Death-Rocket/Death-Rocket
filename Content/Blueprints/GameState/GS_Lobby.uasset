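; Lobby game state for DeathRocket that sets up local multiplayer players and turns on invincibility at BeginPlay.
; SpawnPlayers creates a local player per game instance player count, then possesses the DRPlayerChar actors found in the level by index and adds the Enhanced Input mapping context.
; SetTeam applies the game instance's team array to those characters by index through the game mode, but is not called within this graph.
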(event `self.ReceiveBeginPlay`
  (`self.SpawnPlayers`)
  (`self.SetInvincibility` true))

(event `self.ReceiveTick`
  (params (DeltaSeconds :type "Float (single-precision)")))

(fn `GetNbrOfPlayer`
  (returns (value :type Integer64))
  (bind _asdr_game_instance (cast `DR_GameInstance` (`GameplayStatics.GetGameInstance`)))
  (bind _returnvalue (`DR_GameInstance.GetNbrOfPlayer` _asdr_game_instance))
  (return (`KismetMathLibrary.Conv_IntToInt64` _returnvalue)))

(fn `SetTeam`
  (bind _asdr_game_instance (cast `DR_GameInstance` (`GameplayStatics.GetGameInstance`)))
  (bind _asdeath_rocket_game_mode_base (cast `DeathRocketGameModeBase` (`GameplayStatics.GetGameMode`)))
  (set `self. Death Rocket Game Mode Base` _asdeath_rocket_game_mode_base)
  (bind _returnvalue (`DR_GameInstance.GetTeamArray` _asdr_game_instance))
  (if (`KismetArrayLibrary.Array_IsNotEmpty` _returnvalue)
    (bind _outactors (`GameplayStatics.GetAllActorsOfClass` "/Script/DeathRocket.DRPlayerChar"))
    (for (_array_element _array_index) _outactors
      (`DRPlayerChar.SetTeam` _array_element (`self. Death Rocket Game Mode Base`) (`|GetArrayItem` _returnvalue _array_index)))))

(fn `SpawnPlayers`
  (locals (Index :type Integer))
  (bind _value (`self.GetNbrOfPlayer`))
  (bind _returnvalue (`KismetMathLibrary.Conv_Int64ToInt` (- _value 1)))
  (for _index (range (+ _returnvalue 1))
    (`GameplayStatics.CreatePlayer` _index))
  (bind _outactors (`GameplayStatics.GetAllActorsOfClass` "/Script/DeathRocket.DRPlayerChar"))
  (for _index_2 (range (+ _returnvalue 1))
    (bind _returnvalue_2 (`GameplayStatics.GetPlayerController` _index_2))
    (`Controller.Possess` _returnvalue_2 (`PawnMovementComponent.GetPawnOwner` (`Character.CharacterMovement` (`|GetArrayItem` _outactors _index_2))))
    (message `EnhancedInputSubsystemInterface.AddMappingContext` (pcsubsystem `EnhancedInputLocalPlayerSubsystem` _returnvalue_2) "/Game/Settings/Inputs/DRInputMappingContext.DRInputMappingContext" 0 (struct))))

(fn `UserConstructionScript`)