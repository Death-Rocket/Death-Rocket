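; Game state for the Classic mode that sets up local multiplayer players and their teams at BeginPlay.
; Creates one local player per count from DR_GameInstance, adds the Enhanced Input mapping, then possesses existing DRPlayerChar actors by index.
; Team IDs from the game instance's array are assigned to characters in actor-list order.
; A separate function spawns a replacement pawn at a team respawn point and sets its team.
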(event `self.ReceiveBeginPlay`
  (`self.SpawnPlayers`)
  (`self.SetTeam`))

(event `self.ReceiveTick`
  (params (DeltaSeconds :type "Float (single-precision)")))

(fn `GetNbrOfPlayer`
  (returns (value :type Integer))
  (bind _asdr_game_instance (cast `DR_GameInstance` (`GameplayStatics.GetGameInstance`)))
  (bind _returnvalue (`DR_GameInstance.GetNbrOfPlayer` _asdr_game_instance))
  (return _returnvalue))

(fn `SetTeam`
  (bind _asdr_game_instance (cast `DR_GameInstance` (`GameplayStatics.GetGameInstance`)))
  (bind _asdeath_rocket_game_mode_base (cast `DeathRocketGameModeBase` (`GameplayStatics.GetGameMode`)))
  (set `self. Death Rocket Game Mode Base` _asdeath_rocket_game_mode_base)
  (bind _returnvalue (`DR_GameInstance.GetTeamArray` _asdr_game_instance))
  (if (`KismetArrayLibrary.Array_IsNotEmpty` _returnvalue)
    (bind _outactors (`GameplayStatics.GetAllActorsOfClass` "/Script/DeathRocket.DRPlayerChar"))
    (for (_array_element _array_index) _outactors
      (`DRPlayerChar.SetTeam` _array_element (`self. Death Rocket Game Mode Base`) (`|GetArrayItem` _returnvalue _array_index)))))

(fn `Spawn New Player Pawn`
  (params (TeamId :type Integer) (PlayerClass :type "DRCharacter Class Reference") (PlayerContoller :type "/Game/Blueprints/PlayerController/PC_Player Object Reference"))
  (returns (DrCharacter :type "DRCharacter Object Reference"))
  (bind _returnvalue (`self.GetRespawnPoint` TeamId))
  (bind _returnvalue_2 (`|SpawnActorFromClass` PlayerClass _returnvalue "AdjustIfPossibleButAlwaysSpawn" "MultiplyWithRoot" PlayerContoller null))
  (`DRCharacter.SetTeam` _returnvalue_2 null TeamId)
  (return _returnvalue_2))

(fn `SpawnPlayers`
  (locals (Index :type Integer))
  (`|ExecutionSequence`
    (:`then_0`
      ;[1 1 1] CreatePlayer
      (bind _value (`self.GetNbrOfPlayer`))
      (for _index (range (+ (`KismetMathLibrary.Conv_Int64ToInt` (- _value 1)) 1))
        (bind _output_get (set `local.Index` _index))
        (`GameplayStatics.CreatePlayer` _output_get)))
    (:`then_1`
      ;[1 1 1] Set PlayerLocal
      (bind _outactors (`GameplayStatics.GetAllActorsOfClass` "/Script/Engine.PlayerController"))
      (for (_array_element _array_index) _outactors
        (`GameplayStatics.SetPlayerControllerID` _array_element _array_index)
        (`EnhancedInputSubsystemInterface.AddMappingContext` (pcsubsystem `EnhancedInputLocalPlayerSubsystem` _array_element) "/Game/Settings/Inputs/IMP_PlayerController.IMP_PlayerController" 1 (struct))))
    (:`then_2`
      ;[1 1 1] PossePawn
      (bind _value_2 (`self.GetNbrOfPlayer`))
      (bind _outactors_2 (`GameplayStatics.GetAllActorsOfClass` "/Script/DeathRocket.DRPlayerChar"))
      (for _index_2 (range _value_2)
        (bind _output_get_2 (set `local.Index` _index_2))
        (`Controller.Possess` (`GameplayStatics.GetPlayerController` _output_get_2) (`PawnMovementComponent.GetPawnOwner` (`Character.CharacterMovement` (`|GetArrayItem` _outactors_2 _index_2))))))))

(fn `UserConstructionScript`)