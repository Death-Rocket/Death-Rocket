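; A buff pickup actor that grants a random buff to the player who touches it.
; The construction script picks one class from BuffArray, and the static mesh spins each tick.
; When a DRPlayerChar overlaps the sphere, it spawns that buff at the character's transform and passes it to the PC_Player controller's AddBuff.
; The pickup destroys itself only if AddBuff succeeds.
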(event `self.ReceiveBeginPlay`)

(event `self.ReceiveTick`
  (params (DeltaSeconds :type "Float (single-precision)"))
  ;[1 1 1] Make The Thing Rotate
  (`SceneComponent.K2_AddLocalRotation` (`self.StaticMesh`) (struct :`Pitch` 1.0 :`Yaw` 1.0 :`Roll` 1.0) false false))

(event `self.Sphere.OnComponentBeginOverlap`
  (params (OverlappedComponent :type "PrimitiveComponent Object Reference") (OtherActor :type "Actor Object Reference") (OtherComp :type "PrimitiveComponent Object Reference") (OtherBodyIndex :type Integer) (bFromSweep :type Boolean) (SweepResult :type "HitResult Structure (by ref)"))
  (`self.OnPlayerOverLap` OtherActor))

(fn `OnPlayerOverLap`
  (params (ObjectOverlap :type "Object Object Reference"))
  (bind _asdrplayer_char (cast `DRPlayerChar` ObjectOverlap))
  (bind _aspc_player (cast `/Game/Blueprints/PlayerController/PC_Player` (`PlayerState.GetPlayerController` (`Pawn.PlayerState` _asdrplayer_char))))
  (bind _returnvalue (`|SpawnActorFromClass` (`self.BuffClass`) (`self.GetTransform` _asdrplayer_char) "AlwaysSpawn" "MultiplyWithRoot" null null))
  (bind _hasbeenadded (`/Game/Blueprints/PlayerController/PC_Player.Add Buff` _aspc_player _returnvalue))
  (if _hasbeenadded
    (`self.K2_DestroyActor`)))

(fn `UserConstructionScript`
  (bind _buffarray (`self.BuffArray`))
  (set `self.BuffClass` (`|GetArrayItem` _buffarray (`KismetMathLibrary.RandomInteger` (`KismetArrayLibrary.Array_Length` _buffarray)))))