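; Player controller for a team-based local player, managing pawn setup, buffs, ultimate charge, HUD and pause menu.
; On possess it applies the GameInstance's team and ultimate choice to the pawn, then once creates the widgets and grants a base rocket buff.
; Inputs cycle and use buffs, while kill and ammo events update the HUD.
; PossesNewPawn respawns the saved pawn class through GS_Classic and possesses it.
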(event `self.ReceiveBeginPlay`)

(event `self.ReceivePossess`
  (params (PossessedPawn :type "Pawn Object Reference"))
  (`self.GetPlayerPawn`)
  (`self.InitPawnMaterial`)
  (`self.SetUltPawn` (`self.GetControlledPlayerPawn`))
  (`/Engine/EditorBlueprintResources/StandardMacros.DoOnce` false
    (:`Completed`
      (`self.Init Ui`)
      ;[1 1 1] Add base Reset Buff
      (bind _returnvalue (`|SpawnActorFromClass` "/Game/Blueprints/Buff/Child/BP_BuffBaseRocket.BP_BuffBaseRocket_C" (`KismetMathLibrary.MakeTransform` (0.0 0.0 0.0)) "Undefined" "MultiplyWithRoot" null null))
      (`self.Add Buff` _returnvalue)
      (`/Engine/EditorBlueprintResources/StandardMacros.IsValid` (`self.PauseMenue`)
        (:`Is Not Valid`
          (bind _returnvalue_2 (`|CreateWidget` "/Game/Blueprints/UI/WB_PlayerPauseMenue.WB_PlayerPauseMenue_C"))
          (set `self.PauseMenue` _returnvalue_2))))))

(event `EnhancedInput|/Game/Settings/Inputs/Actions/PlayerController/BuffRight`
  (params (ActionValue :type Boolean) (ElapsedSeconds :type "Float (double-precision)") (TriggeredSeconds :type "Float (double-precision)") (InputAction :type "InputAction Object Reference" :default "/Game/Settings/Inputs/Actions/PlayerController/BuffRight.BuffRight"))
  ;[1 1 1] BuffInput
  (:`Completed`
    (`self.OnPlayerChooseBuff` (+ (`self.BuffIndex`) 1))))

(event `EnhancedInput|/Game/Settings/Inputs/Actions/PlayerController/BuffLeft`
  (params (ActionValue :type Boolean) (ElapsedSeconds :type "Float (double-precision)") (TriggeredSeconds :type "Float (double-precision)") (InputAction :type "InputAction Object Reference" :default "/Game/Settings/Inputs/Actions/PlayerController/BuffLeft.BuffLeft"))
  ;[1 1 1] BuffInput
  (:`Completed`
    (`self.OnPlayerChooseBuff` (- (`self.BuffIndex`) 1))))

(event `self.SetUltPercent`
  (params (percent :type "Float (single-precision)"))
  ;[1 1 1] Ultimate
  (if (<= percent 1.0)
    (`/Game/Blueprints/UI/WB_PlayerUI.SetPercent` (`self.UltBar`) percent)))

(event `EnhancedInput|/Game/Settings/Inputs/Actions/PlayerController/BuffUse`
  (params (ActionValue :type Boolean) (ElapsedSeconds :type "Float (double-precision)") (TriggeredSeconds :type "Float (double-precision)") (InputAction :type "InputAction Object Reference" :default "/Game/Settings/Inputs/Actions/PlayerController/BuffUse.BuffUse"))
  ;[1 1 1] BuffInput
  (:`Completed`
    (`self.OnPlayerPressUseBuff`)))

(event `OnPawnDoKill`
  ;[1 1 1] Ultimate
  (`self.Add Percent to Ult Bar` (`self.UltPercentBonusOnKill`)))

(event `EnhancedInput|/Game/Settings/Inputs/Actions/PlayerController/PopMenue`
  (params (ActionValue :type Boolean) (ElapsedSeconds :type "Float (double-precision)") (TriggeredSeconds :type "Float (double-precision)") (InputAction :type "InputAction Object Reference" :default "/Game/Settings/Inputs/Actions/PlayerController/PopMenue.PopMenue"))
  ;[1 1 1] Menue
  (:`Completed`
    (if (not (`Widget.IsVisible` (`self.PauseMenue`)))
      (`UserWidget.AddToPlayerScreen` (`self.PauseMenue`) 0))))

(event `OnNbrBullerUpdate`
  ;[1 1 1] On Reload Ui Event
  (bind _returnvalue (`DRCharacter.GetCurrentAmmo` (`self.GetControlledPlayerPawn`)))
  (`/Game/Blueprints/UI/WB_PlayerUI.Update Ammo Amout` (`self.UltBar`) (- _returnvalue 1)))

(event `OnPawnReload`
  ;[1 1 1] On Reload Ui Event
  (bind _returnvalue (`DRCharacter.GetMaxAmmo` (`self.GetControlledPlayerPawn`)))
  (`/Game/Blueprints/UI/WB_PlayerUI.Update Ammo Amout` (`self.UltBar`) _returnvalue))

(fn `Add Buff`
  (params (NewBuff :type "DR_Buff Object Reference"))
  (returns (HasBeenAdded :type Boolean))
  (locals (buff :type "DR_Buff Object Reference"))
  (bind _output_get (set `local.buff` NewBuff))
  (bind (_buffindex _returnvalue) (`self.GetBuff` _output_get))
  (if _returnvalue
    (`/Game/Blueprints/UI/WB_PlayerUI.OnGetBuff` (`self.UltBar`) _buffindex (`DR_Buff.BuffImage` (`local.buff`)))
    (return true)
    (else
      (return true))))

(fn `Add Percent to Ult Bar`
  (params (Percent :type "Float (double-precision)"))
  (bind _output_get (set `self.PlayerUltCharge` (`KismetMathLibrary.FClamp` (+ Percent (`self.PlayerUltCharge`)) 0.0 100.0)))
  (`/Game/Blueprints/UI/WB_PlayerUI.SetPercent` (`self.UltBar`) (/ _output_get 100.0)))

(fn `GetControlledPlayerPawn`
  (returns (PlayerPawn :type "DRCharacter Object Reference"))
  (bind _asdrcharacter (cast `DRCharacter` (`self.K2_GetPawn`)))
  (return _asdrcharacter))

(fn `GetPlayerPawn`
  (bind _asdrcharacter (cast `DRCharacter` (`self.K2_GetPawn` (`GameplayStatics.GetPlayerController` (`GameplayStatics.GetPlayerControllerID` self)))))
  (set `self.PlayerClass` (`GameplayStatics.GetObjectClass` _asdrcharacter)))

(fn `GetTeamFromGameInstance`
  (returns (Team :type Integer))
  (bind _asdr_game_instance (cast `DR_GameInstance` (`GameplayStatics.GetGameInstance`)))
  (bind _returnvalue (`DR_GameInstance.GetPlayerGetTeam` _asdr_game_instance (`self.GetPlayerLocalID`)))
  (return _returnvalue))

(fn `Init Ui`
  (if (not (`KismetSystemLibrary.IsValid` (`self.UltBar`)))
    (bind _returnvalue (`|CreateWidget` "/Game/Blueprints/UI/WB_PlayerUI.WB_PlayerUI_C" self))
    (bind _output_get (set `self.UltBar` _returnvalue))
    (bind _returnvalue_2 (`DRCharacter.GetMaxAmmo` (`self.GetControlledPlayerPawn`)))
    (bind _output_get_2 (set `/Game/Blueprints/UI/WB_PlayerUI.MaxAmmo` _returnvalue_2 _output_get))
    (`/Game/Blueprints/UI/WB_PlayerUI.Update Ammo Amout` _output_get _output_get_2)
    (`UserWidget.AddToPlayerScreen` _output_get 0)))

(fn `InitPawnMaterial`
  (bind _asdrplayer_char (cast `DRPlayerChar` (`self.K2_GetPawn`)))
  (bind _team (`self.GetTeamFromGameInstance`))
  (bind _asgm_classic (cast `/Game/Blueprints/GameMode/GM_Classic` (`GameplayStatics.GetGameMode`)))
  (`/Game/Blueprints/GameMode/GM_Classic.SetTeamMaterial` _asgm_classic (`Character.Mesh` _asdrplayer_char) _team))

(fn `OnPlayerChooseBuff`
  (params (NewValue :type Integer))
  (`self.UpdateBuffIndex` NewValue)
  (`/Game/Blueprints/UI/WB_PlayerUI.OnSelectBuffChange` (`self.UltBar`) (`self.BuffIndex`)))

(fn `OnPlayerPressUseBuff`
  (`self.UseBuff` (`self.BuffIndex`))
  (`/Game/Blueprints/UI/WB_PlayerUI.OnConsumeBuff` (`self.UltBar`) 0 (`self.buffs`)))

(fn `PossesNewPawn`
  (locals (NewPawn :type "DRCharacter Object Reference"))
  (bind _team (`self.GetTeamFromGameInstance`))
  (bind _asgs_classic (cast `/Game/Blueprints/GameState/GS_Classic` (`GameplayStatics.GetGameState`)))
  (bind _drcharacter (`/Game/Blueprints/GameState/GS_Classic.Spawn New Player Pawn` _asgs_classic _team (`self.PlayerClass`) self))
  (if (`KismetSystemLibrary.IsValid` _drcharacter)
    (set `local.NewPawn` _drcharacter)
    (`self.UnPossess`)
    (`self.Possess` (`local.NewPawn`))
    (else
      (`KismetSystemLibrary.PrintText` "ON CONTROLLER TRY GET PAWN INVALID"))))

(fn `SetUltPawn`
  (params (PlayerPawn :type "DRCharacter Object Reference"))
  (bind _returnvalue (`self.GetPlayerLocalID`))
  (bind _asdr_game_instance (cast `DR_GameInstance` (`GameplayStatics.GetGameInstance`)))
  (bind _asdrplayer_char (cast `DRPlayerChar` PlayerPawn))
  (if (!= _returnvalue -1)
    (bind _returnvalue_2 (`DR_GameInstance.GetPlayerUltimate` _asdr_game_instance _returnvalue))
    (`DRPlayerChar.SetPawnUlt` _asdrplayer_char _returnvalue_2)))

(fn `UpdateBuffIndex`
  (params (NewIndex :type Integer))
  ;[1 1 1] Set index Zero f overflow
  (if (>= NewIndex (`self.maxBuffNbr`))
    (set `self.BuffIndex` 0)
    (else
      ;[1 1 1] Set to max if negative
      (if (< NewIndex 0)
        (set `self.BuffIndex` (- (`self.maxBuffNbr`) 1))
        (else
          (set `self.BuffIndex` NewIndex))))))

(fn `UserConstructionScript`)