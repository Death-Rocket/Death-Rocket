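; BP_SelectTeamBox is a trigger volume that assigns a player to a team while they stand inside it.
; When a DRPlayerChar begins overlapping the Box, it sets the character's team to the box's TeamValue and has GM_Classic apply that team's material to the character mesh.
; Leaving the box resets the team to -1 and updates the mesh material the same way.
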(event `self.ReceiveActorBeginOverlap`
  (params (OtherActor :type "Actor Object Reference")))

(event `self.Box.OnComponentBeginOverlap`
  (params (OverlappedComponent :type "PrimitiveComponent Object Reference") (OtherActor :type "Actor Object Reference") (OtherComp :type "PrimitiveComponent Object Reference") (OtherBodyIndex :type Integer) (bFromSweep :type Boolean) (SweepResult :type "HitResult Structure (by ref)"))
  (bind _teamvalue (`self.TeamValue`))
  (bind _asdrplayer_char (cast `DRPlayerChar` OtherActor))
  (`DRPlayerChar.SetTeam` _asdrplayer_char (`GameplayStatics.GetGameMode`) _teamvalue)
  (bind _asgm_classic (cast `/Game/Blueprints/GameMode/GM_Classic` (`GameplayStatics.GetGameMode`)))
  (`/Game/Blueprints/GameMode/GM_Classic.SetTeamMaterial` _asgm_classic (`Character.Mesh` _asdrplayer_char) _teamvalue))

(event `self.Box.OnComponentEndOverlap`
  (params (OverlappedComponent :type "PrimitiveComponent Object Reference") (OtherActor :type "Actor Object Reference") (OtherComp :type "PrimitiveComponent Object Reference") (OtherBodyIndex :type Integer))
  (bind _asdrplayer_char (cast `DRPlayerChar` OtherActor))
  (`DRPlayerChar.SetTeam` _asdrplayer_char (`GameplayStatics.GetGameMode`) -1)
  (bind _asgm_classic (cast `/Game/Blueprints/GameMode/GM_Classic` (`GameplayStatics.GetGameMode`)))
  (`/Game/Blueprints/GameMode/GM_Classic.SetTeamMaterial` _asgm_classic (`Character.Mesh` _asdrplayer_char) -1))

(fn `UserConstructionScript`)