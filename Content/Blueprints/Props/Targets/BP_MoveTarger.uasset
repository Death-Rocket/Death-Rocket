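; BP_MoveTarger is a target prop that moves continuously along its own spline.
; BeginPlay stores the starting location; each Tick advances a distance by Speed and resets it to zero past the spline's end, looping the motion.
; The root component takes the spline's local-space location offset by that start position, plus the spline's rotation, keeping its scale.
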(event `self.ReceiveBeginPlay`
  (set `self.BasePos` (`self.K2_GetActorLocation`)))

(event `self.ReceiveTick`
  (params (DeltaSeconds :type "Float (single-precision)"))
  (bind (_returnvalue_location _returnvalue_rotation) (`KismetMathLibrary.BreakTransform` (`SplineComponent.GetTransformAtDistanceAlongSpline` (`self.Spline`) (`self.Distance Along Spline`) "Local" false)))
  (set `self.Distance Along Spline` (+ (* DeltaSeconds (`self.Speed`)) (`self.Distance Along Spline`)))
  (`SceneComponent.K2_SetRelativeTransform` (`self.DefaultSceneRoot`) (`KismetMathLibrary.MakeTransform` (+ _returnvalue_location (`self.BasePos`)) _returnvalue_rotation (`SceneComponent.RelativeScale3D` (`self.DefaultSceneRoot`))) false false)
  (if (> (`self.Distance Along Spline`) (`SplineComponent.GetSplineLength` (`self.Spline`)))
    (set `self.Distance Along Spline` 0.0)))

(fn `UserConstructionScript`)