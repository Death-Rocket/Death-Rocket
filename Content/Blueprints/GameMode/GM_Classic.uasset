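; GM_Classic is the game mode for the Classic mode, handling match start and end plus team visuals.
; On begin play it briefly shows WB_StartGameWidget, then tells GS_Classic to pop the game mode overlay.
; Game end opens the Menu level, and SetTeamMaterial applies a team-specific overlay material to a given mesh.
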(event `self.ReceiveBeginPlay`
  (`self.OnGameBegin`))

(event `self.OnGameBegin`
  (bind _returnvalue (`|CreateWidget` "/Game/Blueprints/UI/WB_StartGameWidget.WB_StartGameWidget_C"))
  (`UserWidget.AddToViewport` _returnvalue 0)
  (`KismetSystemLibrary.Delay` 0.5)
  (`Widget.RemoveFromParent` _returnvalue)
  (bind _asgs_classic (cast `/Game/Blueprints/GameState/GS_Classic` (`GameplayStatics.GetGameState`)))
  (`DR_GameState.PopGameModeOverlay` _asgs_classic))

(event `self.OnGameEnd`
  (params (teamID :type Integer))
  (`GameplayStatics.OpenLevelBySoftObjectPtr` "/Game/Map/Menu.Menu"))

(fn `SetTeamMaterial`
  (params (mesh :type "SkeletalMeshComponent Object Reference") (teamId :type Integer))
  (bind _returnvalue (`self.GetOverlayMaterialColor` teamId))
  (`MeshComponent.SetOverlayMaterial` mesh _returnvalue))

(fn `UserConstructionScript`)