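; Game mode for Classic Domination that handles the end of a match.
; OnGameEnd, meant to be called by the GameState, receives the winning team ID, stops all players, shows the WB_EngGame winner widget, then loads the Menu level after a short delay.
; An invalid team ID only prints an error message.
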(event `self.OnGameEnd`
  (params (teamID :type Integer))
  ;[1 1 1] Should Be calld by the GameState
  (if (!= teamID -1)
    (`self.AllPlayerStopPlay`)
    (bind _returnvalue (`|CreateWidget` "/Game/Blueprints/UI/WB_EngGame.WB_EngGame_C"))
    (`/Game/Blueprints/UI/WB_EngGame.SetViewportWinerTeam` _returnvalue teamID)
    (`UserWidget.AddToViewport` _returnvalue 0)
    (`KismetSystemLibrary.Delay` 2.0)
    (`GameplayStatics.OpenLevelBySoftObjectPtr` "/Game/Map/Menu.Menu")
    (else
      (`KismetSystemLibrary.PrintText` "InValid WiningTeam ID GM_Domimation"))))

(fn `UserConstructionScript`
  (`parent.UserConstructionScript`))