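; BP_HomingRocket is a rocket that locks onto characters from an opposing team.
; When an actor overlaps it, it casts to DRCharacter and compares that character's team with its own MTeamNb.
; On a mismatch, it sets the character's mesh as the Movement component's homing target, then triggers the blink on its BP_BlinkingSphere child actor.
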(event `self.ReceiveBeginPlay`)

(event `self.ReceiveActorBeginOverlap`
  (params (OtherActor :type "Actor Object Reference"))
  ;[1 0.2083 0.9651] Active Homing
  (bind _asdrcharacter (cast `DRCharacter` OtherActor))
  (bind _returnvalue (`DRCharacter.GetTeam` _asdrcharacter))
  (if (!= _returnvalue (`self.mTeamNb`))
    (set `ProjectileMovementComponent.HomingTargetComponent` (`Character.Mesh` _asdrcharacter) (`self.Movement`))
    ;[1 0.1208 0.3216] Activate blink
    (bind _asbp_blinking_sphere (cast `/Game/Blueprints/Rockets/BP_BlinkingSphere` (`ChildActorComponent.ChildActor` (`self.BP_BlinkingSphere`))))
    (`/Game/Blueprints/Rockets/BP_BlinkingSphere.ActivateBlink` _asbp_blinking_sphere)))

(fn `UserConstructionScript`)