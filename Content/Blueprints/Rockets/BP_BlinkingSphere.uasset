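; BP_BlinkingSphere is a sphere that blinks with a red point light when activated.
; It stores the light's initial intensity on BeginPlay and starts with the light off.
; ActivateBlink runs a Delay-based loop that alternates laser pointer and grey materials along with the light, using separate on and off durations.
; DeActivateBlink clears the Active flag that sustains the loop and immediately restores the unlit grey look.
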(event `self.ReceiveBeginPlay`
  (bind _redpointlight (`self.RedPointLight`))
  ;[1 1 1] Setup base values
  (set `self.BaseIntensity` (`LightComponentBase.Intensity` _redpointlight))
  (`LightComponent.SetIntensity` _redpointlight 0.0))

(event `ActivateBlink`
  ;[0 1 0.1703] Activation
  (set `self.Active` true)
  (`PrimitiveComponent.SetMaterial` (`self.Sphere`) 0 "/Engine/VREditor/LaserPointer/LaserPointerMaterial.LaserPointerMaterial" :!label _label)
  (`LightComponent.SetIntensity` (`self.RedPointLight`) (`self.BaseIntensity`))
  (`KismetSystemLibrary.Delay` (`self.BlinkingOnDuration`))
  (`PrimitiveComponent.SetMaterial` (`self.Sphere`) 0 "/Engine/EditorMeshes/ColorCalibrator/M_GreyBall.M_GreyBall")
  (`LightComponent.SetIntensity` (`self.RedPointLight`) 0.0)
  (`KismetSystemLibrary.Delay` (`self.BlinkingOffDuration`))
  (if (`self.Active`)
    (goto _label)))

(event `DeActivateBlink`
  ;[1 0.04671 0] Deactivation
  (set `self.Active` false)
  (`PrimitiveComponent.SetMaterial` (`self.Sphere`) 0 "/Engine/EditorMeshes/ColorCalibrator/M_GreyBall.M_GreyBall")
  (`LightComponent.SetIntensity` (`self.RedPointLight`) 0.0))

(fn `UserConstructionScript`)