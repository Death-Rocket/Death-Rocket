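; BP_TripleRocket is a rocket that turns one shot into a three-rocket spread.
; One tick after BeginPlay, it spawns two BP_OneOfTripleRocket actors slightly ahead of itself, yawed to either side by AngleBetween2Rockets.
; It passes its character owner to both side rockets and registers itself as the original rocket on all three.
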(event `self.ReceiveBeginPlay`
  (bind _returnvalue (`KismetMathLibrary.ComposeRotators` (`KismetMathLibrary.MakeRotator` 0.0 0.0 (`self.AngleBetween2Rockets`)) (`self.K2_GetActorRotation`)))
  (`self.SetOriginalRocket` self)
  (`KismetSystemLibrary.DelayUntilNextTick`)
  (bind _returnvalue_2 (`self.GetCharacterOwner`))
  (bind _returnvalue_3 (`|SpawnActorFromClass` "/Game/Blueprints/Rockets/BP_OneOfTripleRocket.BP_OneOfTripleRocket_C" (`KismetMathLibrary.MakeTransform` (+ (`self.K2_GetActorLocation`) (* (`KismetMathLibrary.GetForwardVector` _returnvalue) (100.0 100.0 100.0))) _returnvalue) "AdjustIfPossibleButAlwaysSpawn" "MultiplyWithRoot" null self))
  (bind _result (`/Engine/EditorBlueprintResources/StandardMacros.NegateFloat` (`self.AngleBetween2Rockets`))
    (:`  `
      (bind _returnvalue_4 (`KismetMathLibrary.ComposeRotators` (`KismetMathLibrary.MakeRotator` 0.0 0.0 _result) (`self.K2_GetActorRotation`)))
      (bind _returnvalue_5 (`|SpawnActorFromClass` "/Game/Blueprints/Rockets/BP_OneOfTripleRocket.BP_OneOfTripleRocket_C" (`KismetMathLibrary.MakeTransform` (+ (`self.K2_GetActorLocation`) (* (`KismetMathLibrary.GetForwardVector` _returnvalue_4) (100.0 100.0 100.0))) _returnvalue_4) "AdjustIfPossibleButAlwaysSpawn" "MultiplyWithRoot" null self))
      (`self.SetCharacterOwner` _returnvalue_5 _returnvalue_2)
      (`self.SetCharacterOwner` _returnvalue_3 _returnvalue_2)
      (`self.SetOriginalRocket` _returnvalue_3 self)
      (`self.SetOriginalRocket` _returnvalue_5 self))))

(fn `UserConstructionScript`)