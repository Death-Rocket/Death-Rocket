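; BP_Player_Wraith is the Wraith player pawn, handling animation and feedback for combat events.
; Shooting plays a random montage, and reloading plays a montage that stops on completion.
; Death, kill, ammo-spend and reload-finished events are forwarded to PC_Player, which possesses a new pawn on death.
; Damage assigns a dynamic screen-damage material instance to the follow camera's post-process settings.
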(event `self.ReceiveBeginPlay`)

(event `self.OnShoot`
  ;[1 1 1] OnShootAnim
  (`|PlayMontage` (`self.Mesh`) (`KismetArrayLibrary.Array_Random` (`self.ShootAnimMontage`))))

(event `self.OnDie`
  ;[1 1 1] On Die
  (bind _aspc_player (cast `/Game/Blueprints/PlayerController/PC_Player` (`self.GetController`)))
  (`/Game/Blueprints/PlayerController/PC_Player.PossesNewPawn` _aspc_player))

(event `self.OnReloaded`
  ;[1 1 1] On Reload
  (`/Game/Blueprints/PlayerController/PC_Player.OnPawnReload` (cast `/Game/Blueprints/PlayerController/PC_Player` (`self.GetController`) :!pure true))
  (`self.StopAnimMontage` (`self.mReloadAnimMontage`)))

(event `self.OnDamage`
  (`self.ActivateDamageScreen`))

(event `self.OnReload`
  ;[1 1 1] On Reload
  (`|PlayMontage` (`self.Mesh`) (`self.mReloadAnimMontage`)))

(event `self.OnSpendAmmo`
  ;[1 1 1] On Reload
  (`/Game/Blueprints/PlayerController/PC_Player.OnNbrBullerUpdate` (cast `/Game/Blueprints/PlayerController/PC_Player` (`self.GetController`) :!pure true)))

(event `self.OnKill`
  ;[1 1 1] On Kill
  (bind _aspc_player (cast `/Game/Blueprints/PlayerController/PC_Player` (`self.GetController`)))
  (`/Game/Blueprints/PlayerController/PC_Player.OnPawnDoKill` _aspc_player))

(fn `ActivateDamageScreen`
  (bind _returnvalue (`KismetMaterialLibrary.CreateDynamicMaterialInstance` "/Game/Material/M_ScreenDamage_Inst.M_ScreenDamage_Inst"))
  (bind _output_get (set `self.Damage Screen` _returnvalue))
  (set `CameraComponent.PostProcessSettings` (make `PostProcessSettings` :`AutoExposureMinBrightness` 1.0 :`AutoExposureMaxBrightness` 1.0 :`WeightedBlendables` (make `WeightedBlendables` (`|MakeArray` (make `WeightedBlendable` 1.0 _output_get)))) (`self.mFollowCamera`)))

(fn `PlayRandomAnimation`)

(fn `UserConstructionScript`)