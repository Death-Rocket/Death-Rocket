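; Test player Blueprint that sets up the player's aim reticle and team and shows a screen damage effect.
; On BeginPlay it adds the WB_AimReticle widget to the player screen and assigns a team ID.
; OnDamage creates a new dynamic instance of the screen damage material and rebuilds the follow camera's post-process settings with it as a full-weight blendable.
; Nothing here fades or clears the effect.
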(event `self.ReceiveBeginPlay`
  (bind _returnvalue (`|CreateWidget` "/Game/Blueprints/Player/WB_AimReticle.WB_AimReticle_C"))
  (`UserWidget.AddToPlayerScreen` _returnvalue 0)
  (`self.SetTeam` null 2))

(event `self.OnDamage`
  (`self.ActivateDamageScreen`))

(fn `ActivateDamageScreen`
  (bind _returnvalue (`KismetMaterialLibrary.CreateDynamicMaterialInstance` "/Game/Material/M_ScreenDamage_Inst.M_ScreenDamage_Inst"))
  (bind _output_get (set `self.DamageScreen` _returnvalue))
  (set `CameraComponent.PostProcessSettings` (make `PostProcessSettings` :`AutoExposureMinBrightness` 1.0 :`AutoExposureMaxBrightness` 1.0 :`WeightedBlendables` (make `WeightedBlendables` (`|MakeArray` (make `WeightedBlendable` 1.0 _output_get)))) (`self.mFollowCamera`)))

(fn `UserConstructionScript`)